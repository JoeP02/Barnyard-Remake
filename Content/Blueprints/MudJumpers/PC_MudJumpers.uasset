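; Player controller for the Mud Jumpers game that handles jump input and sets up the HUD.
; On BeginPlay it adds the IM_MudJumpers Enhanced Input mapping context for player 0 and adds the WBP_MJ_HUD widget to the viewport.
; The jump action starts and stops jumping on the possessed Character, printing debug success or fail messages.
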(event `EnhancedInput|/Game/Input/MudJumpers/IA_MJ_Jump`
  (params (ActionValue :type Boolean) (ElapsedSeconds :type "Float (double-precision)") (TriggeredSeconds :type "Float (double-precision)") (InputAction :type "InputAction Object Reference" :default "/Game/Input/MudJumpers/IA_MJ_Jump.IA_MJ_Jump"))
  (bind _returnvalue (`self.K2_GetPawn`))
  (:`Started`
    (bind _ascharacter (cast `Character` _returnvalue)
      (:`then`
        (`Character.Jump` _ascharacter)
        (`KismetSystemLibrary.PrintString` "Success" :!label _label))
      (:`CastFailed`
        (`KismetSystemLibrary.PrintString` "Fail" :!label _label_2))))
  (:`Completed`
    (bind _ascharacter_2 (cast `Character` _returnvalue)
      (:`then`
        (`Character.StopJumping` _ascharacter_2)
        (goto _label))
      (:`CastFailed`
        (goto _label_2)))))

(event `CharacterSetup`
  (`EnhancedInputSubsystemInterface.AddMappingContext` (pcsubsystem `EnhancedInputLocalPlayerSubsystem` (`GameplayStatics.GetPlayerController` 0)) "/Game/Input/IM_MudJumpers.IM_MudJumpers" 0 (struct))
  (bind _returnvalue (`|CreateWidget` "/Game/UI/MudJumpers/WBP_MJ_HUD.WBP_MJ_HUD_C"))
  (`UserWidget.AddToViewport` _returnvalue 0)
  (`KismetSystemLibrary.PrintString` "SetUp"))

(event `self.ReceiveBeginPlay`
  (`self.CharacterSetup`))

(fn `UserConstructionScript`)