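; GI_Barnyard, apparently the game instance, unlocks follow-up quests when a quest is completed.
; OnQuestComplete finds the finished quest's class in the GameQuests table and walks that entry's NewQuests.
; Each new quest requires all its QuestsToDo in the player character's BPQuestTracker completed list.
; Eligible quests are handed to the first actor of their QuestGiver class by setting ActiveDialogue and HasQuest.
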(event `On Quest Complete`
  (params (`Current Quest` :type "/Game/Narrative/BarnyardDialogue Object Reference"))
  (for (_array_element _array_index) (`self.Game Quests`)
    (if (== (`/Game/Narrative/QuestData/DA_Quest.Quest` _array_element) (`GameplayStatics.GetObjectClass` `Current Quest`))
      (set `self.Quest Index` _array_index)
      (set `self.Found Quest` true)
      (break)
      (else
        (set `self.Found Quest` false))))
  (if (`self.Found Quest`)
    (bind _asamerican_m_character (cast `/Game/ThirdPerson/Blueprints/AmericanM_Character` (`GameplayStatics.GetPlayerCharacter` 0)))
    (set `self.Player` _asamerican_m_character)
    (for _array_element_2 (`/Game/Narrative/QuestData/DA_Quest.New Quests` (`|GetArrayItem` (`self.Game Quests`) (`self.Quest Index`)))
      (set `self.Can Start Quest` true)
      (for _array_element_3 (`/Game/Narrative/QuestData/DA_Quest.Quests To Do` _array_element_2)
        (if (not (`KismetArrayLibrary.Array_Contains` (`/Game/Blueprints/BP_QuestTracker.Completed Quests` (`/Game/ThirdPerson/Blueprints/AmericanM_Character.BP_QuestTracker` (`self.Player`))) (`/Game/Narrative/QuestData/DA_Quest.Quest` _array_element_3)))
          (set `self.Can Start Quest` false)
          (break)))
      (if (`self.Can Start Quest`)
        (bind _returnvalue (`GameplayStatics.GetActorOfClass` (`/Game/Narrative/QuestData/DA_Quest.Quest Giver` _array_element_2)))
        (set `/Game/ThirdPerson/Blueprints/BP_NPC.ActiveDialogue` (`/Game/Narrative/QuestData/DA_Quest.Quest` _array_element_2) _returnvalue)
        (set `/Game/ThirdPerson/Blueprints/BP_NPC.Has Quest` true _returnvalue)))))