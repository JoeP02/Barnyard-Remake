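; Recipe pickup actor that teaches the player a recipe when interacted with.
; Overlapping its InteractSphere sets the player character's interact widget to this actor's prompt text and shows it, and leaving hides it.
; Interact adds the Recipe to the player's BPRecipeTracker, plays a left-hand pickup montage and destroys the actor immediately.
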(event `/Game/Blueprints/Interfaces/InteractInterface.Interact`
  (bind _asamerican_m_character (cast `/Game/ThirdPerson/Blueprints/Playable/AmericanM_Character_Play` (`GameplayStatics.GetPlayerCharacter` 0)))
  (`KismetArrayLibrary.Array_Add` (`/Game/Blueprints/BP_RecipeTracker.Recipes` (`/Game/ThirdPerson/Blueprints/Playable/AmericanM_Character_Play.BP_RecipeTracker` _asamerican_m_character)) (`self.Recipe`))
  (`Character.PlayAnimMontage` _asamerican_m_character "/Game/Characters/AmericanM/americanM_Anim_Pickup_L_Montage.americanM_Anim_Pickup_L_Montage" 1.0 "None")
  (`self.K2_DestroyActor`))

(event `self.InteractSphere.OnComponentBeginOverlap`
  (params (OverlappedComponent :type "PrimitiveComponent Object Reference") (OtherActor :type "Actor Object Reference") (OtherComp :type "PrimitiveComponent Object Reference") (OtherBodyIndex :type Integer) (bFromSweep :type Boolean) (SweepResult :type "HitResult Structure (by ref)"))
  (bind _asamerican_m_character (cast `/Game/ThirdPerson/Blueprints/Playable/AmericanM_Character_Play` OtherActor))
  (bind _interact_widget (`/Game/ThirdPerson/Blueprints/Playable/AmericanM_Character_Play.Interact Widget` _asamerican_m_character))
  (set `/Game/UI/WBP_Interact.Interact Text` (`self.Interact Text`) _interact_widget)
  (`Widget.SetVisibility` _interact_widget "Visible"))

(event `self.InteractSphere.OnComponentEndOverlap`
  (params (OverlappedComponent :type "PrimitiveComponent Object Reference") (OtherActor :type "Actor Object Reference") (OtherComp :type "PrimitiveComponent Object Reference") (OtherBodyIndex :type Integer))
  (bind _asamerican_m_character (cast `/Game/ThirdPerson/Blueprints/Playable/AmericanM_Character_Play` OtherActor))
  (`Widget.SetVisibility` (`/Game/ThirdPerson/Blueprints/Playable/AmericanM_Character_Play.Interact Widget` _asamerican_m_character) "Hidden"))

(fn `UserConstructionScript`)