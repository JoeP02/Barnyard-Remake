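; GM_Lobby is the lobby Game Mode that tracks joining players and shares the player list with everyone connected.
; On PostLogin it casts the new controller to PC_Lobby and stores it and its PlayerInfo in two arrays.
; After a short delay, it calls UpdatePlayerList on every stored controller with the full info array.
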(event `self.K2_PostLogin`
  (params (NewPlayer :type "PlayerController Object Reference"))
  (bind _aspc_lobby (cast `/Game/Blueprints/Lobby/PC_Lobby` NewPlayer))
  (`KismetArrayLibrary.Array_Add` (`self.ConnectedPlayers`) _aspc_lobby)
  (`KismetArrayLibrary.Array_Add` (`self.ConnectedPlayerInfo`) (`/Game/Blueprints/Lobby/PC_Lobby.PlayerInfo` _aspc_lobby))
  (`KismetSystemLibrary.Delay` 0.2)
  (for _array_element (`self.ConnectedPlayers`)
    (`/Game/Blueprints/Lobby/PC_Lobby.UpdatePlayerList` _array_element (`self.ConnectedPlayerInfo`))))

(fn `UserConstructionScript`)