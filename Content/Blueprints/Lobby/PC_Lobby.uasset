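; Lobby player controller that manages each player's lobby UI, character choice and ready state.
; It creates a host or client widget based on authority and forwards player list updates to it.
; Character changes respawn and possess the new pawn in place, saving the class to GI_Barnyard.
; Possession and ready toggles update PlayerInfo and make GM_Lobby refresh player lists, while being kicked opens the main menu.
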(event `self.ReceiveBeginPlay`
  (`self.CreateMenus`))

(event `CreateMenus`
  (`/Engine/EditorBlueprintResources/ActorMacros.Switch Has Authority`
    (:`Authority`
      (bind _returnvalue (`|CreateWidget` "/Game/UI/Lobby/WBP_LobbyHost.WBP_LobbyHost_C"))
      (bind _output_get (set `self.LobbyWidget` _returnvalue))
      (`UserWidget.AddToViewport` _output_get 0))
    (:`Remote`
      (bind _returnvalue_2 (`|CreateWidget` "/Game/UI/Lobby/WBP_LobbyClient.WBP_LobbyClient_C"))
      (bind _output_get_2 (set `self.LobbyWidget` _returnvalue_2))
      (`UserWidget.AddToViewport` _output_get_2 0))))

(event `UpdatePlayerList`
  (params (PlayerInfo :type "Array of /Game/Blueprints/Lobby/FPlayerInfo Structure (by ref)"))
  (set `self.ConnectedPlayerInfo` PlayerInfo)
  (`/Engine/EditorBlueprintResources/ActorMacros.Switch Has Authority`
    (:`Authority`
      (bind _aswbp_lobby_host (cast `/Game/UI/Lobby/WBP_LobbyHost` (`self.LobbyWidget`)))
      (`/Game/UI/Lobby/WBP_LobbyHost.UpdatePlayerList` _aswbp_lobby_host PlayerInfo))
    (:`Remote`
      (bind _aswbp_lobby_client (cast `/Game/UI/Lobby/WBP_LobbyClient` (`self.LobbyWidget`)))
      (`/Game/UI/Lobby/WBP_LobbyClient.UpdatePlayerList` _aswbp_lobby_client PlayerInfo))))

(event `ChangeCharacter`
  (params (NewCharacter :type "/Game/ThirdPerson/Blueprints/Playable/AmericanM_Character_Play Class Reference"))
  (bind _returnvalue (`self.K2_GetPawn`))
  (bind _output_get (set `self.SpawnTransform` (`self.GetTransform` _returnvalue)))
  (`self.K2_DestroyActor` _returnvalue)
  (bind _returnvalue_2 (`|SpawnActorFromClass` NewCharacter _output_get "Undefined" "OverrideRootScale" null null))
  (`self.Possess` _returnvalue_2)
  (bind _asgi_barnyard (cast `/Game/Blueprints/GI_Barnyard` (`GameplayStatics.GetGameInstance`)))
  (set `/Game/Blueprints/GI_Barnyard.ChosenCharacter` NewCharacter _asgi_barnyard))

(event `SetCharacterClass`
  (params (ChosenCharacter :type "/Game/ThirdPerson/Blueprints/Playable/AmericanM_Character_Play Class Reference"))
  (bind _asgi_barnyard (cast `/Game/Blueprints/GI_Barnyard` (`GameplayStatics.GetGameInstance`)))
  (set `/Game/Blueprints/GI_Barnyard.ChosenCharacter` ChosenCharacter _asgi_barnyard))

(event `SetReadyStatus`
  (bind _playerinfo (`self.PlayerInfo`))
  (setmembers `/Game/Blueprints/Lobby/FPlayerInfo` :`StructRef` _playerinfo :`bIsReady` (not (`.bIsReady_6_5A534F1946DB19090483C3AC9D1392C7` (break `/Game/Blueprints/Lobby/FPlayerInfo` _playerinfo))))
  (bind _asgm_lobby (cast `/Game/Blueprints/Lobby/GM_Lobby` (`GameplayStatics.GetGameMode`)))
  (`/Game/Blueprints/Lobby/GM_Lobby.UpdatePlayerLists` _asgm_lobby))

(event `self.ReceivePossess`
  (params (PossessedPawn :type "Pawn Object Reference"))
  (setmembers `/Game/Blueprints/Lobby/FPlayerInfo` :`StructRef` (`self.PlayerInfo`) :`Character` PossessedPawn)
  (bind _asgm_lobby (cast `/Game/Blueprints/Lobby/GM_Lobby` (`GameplayStatics.GetGameMode`)))
  (`/Game/Blueprints/Lobby/GM_Lobby.UpdatePlayerLists` _asgm_lobby))

(event `KickedFromLobby`
  (`GameplayStatics.OpenLevelBySoftObjectPtr` "/Game/Levels/MainMenu.MainMenu" true "kicked"))

(fn `UserConstructionScript`)