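; BP_SaveGameZone is a world zone where the player saves the game.
; Its capsule overlap shows or removes a WBP_Interact prompt, created at BeginPlay, for the AmericanM_Character_Play character.
; Interact calls SaveGameData on PC_OpenWorld with the hardcoded "save1" slot.
; An ArrowUpDown timeline, played from Tick and restarted on finish, bobs and rotates the EnterIcon.
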(event `self.ReceiveBeginPlay`
  (bind _returnvalue (`|CreateWidget` "/Game/UI/WBP_Interact.WBP_Interact_C" null (`self.InteractText`)))
  (set `self.Interact Widget` _returnvalue))

(event `self.ReceiveTick`
  (params (DeltaSeconds :type "Float (single-precision)"))
  (bind _entericon (`self.EnterIcon`))
  (bind (_direction _upanddown _rotation) (`Timeline|ArrowUpDown` :!label _label)
    (:`Update`
      (`SceneComponent.K2_SetRelativeLocation` _entericon (`KismetMathLibrary.MakeVector` 0.0 0.0 _upanddown) false false)
      (`SceneComponent.K2_SetRelativeRotation` _entericon (`KismetMathLibrary.MakeRotator` 0.0 0.0 _rotation) false false))
    (:`Finished`
      (goto _label :!via `PlayFromStart`))))

(event `/Game/Blueprints/Interfaces/InteractInterface.Interact`
  (bind _aspc_open_world (cast `/Game/PC_OpenWorld` (`Pawn.GetController` (`GameplayStatics.GetPlayerCharacter` 0))))
  (`/Game/PC_OpenWorld.SaveGameData` _aspc_open_world "save1"))

(event `self.Capsule.OnComponentBeginOverlap`
  (params (OverlappedComponent :type "PrimitiveComponent Object Reference") (OtherActor :type "Actor Object Reference") (OtherComp :type "PrimitiveComponent Object Reference") (OtherBodyIndex :type Integer) (bFromSweep :type Boolean) (SweepResult :type "HitResult Structure (by ref)"))
  (cast `/Game/ThirdPerson/Blueprints/Playable/AmericanM_Character_Play` OtherActor)
  (`UserWidget.AddToViewport` (`self.Interact Widget`) 0))

(event `self.Capsule.OnComponentEndOverlap`
  (params (OverlappedComponent :type "PrimitiveComponent Object Reference") (OtherActor :type "Actor Object Reference") (OtherComp :type "PrimitiveComponent Object Reference") (OtherBodyIndex :type Integer))
  (cast `/Game/ThirdPerson/Blueprints/Playable/AmericanM_Character_Play` OtherActor)
  (`Widget.RemoveFromParent` (`self.Interact Widget`)))

(fn `UserConstructionScript`)