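; Base collectable actor that puts its item into the player's inventory when collected.
; The Collect event casts player 0's character to AmericanM_Character and passes the ItemDataComponent's row name and quantity to its InventoryComponent.
; A successful add destroys the actor, while a failed add prints an error and leaves it in the world.
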(event `/Game/Blueprints/Interfaces/CollectableInterface.Collect`
  (bind _itemdatacomponent (`self.ItemDataComponent`))
  (bind (_itemid_datatable _itemid_rowname) (break `DataTableRowHandle` (`/Game/Inventory/ItemDataComponent.ItemID` _itemdatacomponent)))
  (bind _asamerican_m_character (cast `/Game/ThirdPerson/Blueprints/AmericanM_Character` (`GameplayStatics.GetPlayerCharacter` 0)))
  (bind _success (`/Game/Inventory/InventoryComponent.AddToInventory` (`/Game/ThirdPerson/Blueprints/AmericanM_Character.InventoryComponent` _asamerican_m_character) _itemid_rowname (`/Game/Inventory/ItemDataComponent.Quantity` _itemdatacomponent)))
  (if _success
    (`self.K2_DestroyActor`)
    (else
      (`KismetSystemLibrary.PrintString` "Error"))))

(fn `UserConstructionScript`
  (`parent.UserConstructionScript`))