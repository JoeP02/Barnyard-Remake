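; BP_Collectable_Coin is a coin pickup that adds one coin to the player when collected.
; Its Collect event casts player character 0 to AmericanM_Character_Play, calls AddCoins on it, then destroys the coin; a failed cast leaves the coin in place.
; This graph has no active overlap or tick logic, so it does not show what triggers Collect.
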(event `/Game/Blueprints/Interfaces/CollectableInterface.Collect`
  (bind _asamerican_m_character (cast `/Game/ThirdPerson/Blueprints/Playable/AmericanM_Character_Play` (`GameplayStatics.GetPlayerCharacter` 0)))
  (`/Game/ThirdPerson/Blueprints/Playable/AmericanM_Character_Play.AddCoins` _asamerican_m_character 1)
  (`self.K2_DestroyActor`))

(fn `UserConstructionScript`
  (`parent.UserConstructionScript`))