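; BP_WhiteGate is a padlocked double gate the player opens through interaction after a key check, or which opens at BeginPlay when IsOpen is set.
; An overlap trigger shows an interact widget with prompt or no-key text, using CheckGateType to read the character's barnyard key flag.
; Opening destroys padlock and trigger, disables input during the character's montage, and swings both leaves on a timeline after a delay.
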(event `self.ReceiveBeginPlay`
  (bind _returnvalue (`GameplayStatics.GetPlayerController` 0))
  (if (`self.IsOpen`)
    (`ActorComponent.K2_DestroyComponent` (`self.Padlock`) :!label _label)
    (`ActorComponent.K2_DestroyComponent` (`self.GateTrigger`))
    (bind _asamerican_m_character (cast `/Game/ThirdPerson/Blueprints/AmericanM_Character` (`GameplayStatics.GetPlayerCharacter` 0))
      (:`then`
        (`self.DisableInput` _asamerican_m_character _returnvalue)
        (`|PlayMontage` (`Character.Mesh` _asamerican_m_character) "/Game/Characters/AmericanM/americanM_opengate_Montage.americanM_opengate_Montage"
          (:`then`
            (`KismetSystemLibrary.Delay` 1.4)
            (bind (_direction _openanim) (`Timeline|OpenGateAnim` :!label _label_2)
              (:`Update`
                (`SceneComponent.K2_SetRelativeRotation` (`self.Gate_L`) (`KismetMathLibrary.MakeRotator` 0.0 0.0 (* _openanim -1.0)) false false)
                (`SceneComponent.K2_SetRelativeRotation` (`self.GateBits_L`) (`KismetMathLibrary.MakeRotator` 0.0 0.0 (* _openanim -1.0)) false false)
                (`SceneComponent.K2_SetRelativeRotation` (`self.Gate_R`) (`KismetMathLibrary.MakeRotator` 0.0 0.0 _openanim) false false)
                (`SceneComponent.K2_SetRelativeRotation` (`self.GateBits_R`) (`KismetMathLibrary.MakeRotator` 0.0 0.0 _openanim) false false))))
          (:`OnCompleted`
            (`self.EnableInput` _asamerican_m_character _returnvalue))))
      (:`CastFailed`
        (goto _label_2 :!via `PlayFromStart`)))
    (else
      (bind _returnvalue_2 (`|CreateWidget` "/Game/UI/WBP_Interact.WBP_Interact_C" (`GameplayStatics.GetPlayerController` 0) (`self.Interact Text`)))
      (set `self.Interact Widget` _returnvalue_2))))

(event `/Game/Blueprints/Interfaces/InteractInterface.Interact`
  (`self.Open Gate`))

(event `Open Gate`
  (bind _can_open (`self.Check Gate Type`))
  (if _can_open
    (goto _label)))

(event `self.GateTrigger.OnComponentBeginOverlap`
  (params (OverlappedComponent :type "PrimitiveComponent Object Reference") (OtherActor :type "Actor Object Reference") (OtherComp :type "PrimitiveComponent Object Reference") (OtherBodyIndex :type Integer) (bFromSweep :type Boolean) (SweepResult :type "HitResult Structure (by ref)"))
  (bind _interact_widget (`self.Interact Widget`))
  (cast `/Game/ThirdPerson/Blueprints/AmericanM_Character` OtherActor)
  (bind _can_open (`self.Check Gate Type`))
  (if _can_open
    (set `/Game/UI/WBP_Interact.Interact Text` (`self.Interact Text`) _interact_widget)
    (else
      (set `/Game/UI/WBP_Interact.Interact Text` (`self.No Key Text`) _interact_widget)))
  (`UserWidget.AddToViewport` _interact_widget 0))

(event `self.GateTrigger.OnComponentEndOverlap`
  (params (OverlappedComponent :type "PrimitiveComponent Object Reference") (OtherActor :type "Actor Object Reference") (OtherComp :type "PrimitiveComponent Object Reference") (OtherBodyIndex :type Integer))
  (cast `/Game/ThirdPerson/Blueprints/AmericanM_Character` OtherActor)
  (`Widget.RemoveFromParent` (`self.Interact Widget`)))

(fn `Check Gate Type`
  (returns (`Can Open` :type Boolean))
  (bind _asamerican_m_character (cast `/Game/ThirdPerson/Blueprints/AmericanM_Character` (`GameplayStatics.GetPlayerCharacter` 0)))
  (switch `/Game/Enums/E_GateTypes` (`self.Gate Type`)
    (:`NewEnumerator0`
      (return (`/Game/ThirdPerson/Blueprints/AmericanM_Character.HasBarnyardKey` _asamerican_m_character)))))

(fn `UserConstructionScript`)