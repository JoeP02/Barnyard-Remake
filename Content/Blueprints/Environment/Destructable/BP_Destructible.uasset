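; Interactable destructible prop that the player kicks apart to spawn item drops.
; Overlapping its sphere shows the player's interact widget with this prop's text.
; Interact locks player input, plays a kick montage and, after a short delay, hides the object and spawns the configured item count with random scatter.
; Montage completion restores input and destroys the actor; the separate DropItem function is an empty stub.
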(event `/Game/Blueprints/Interfaces/InteractInterface.Interact`
  (bind _returnvalue (`GameplayStatics.GetPlayerController` 0))
  (bind _asamerican_m_character (cast `/Game/ThirdPerson/Blueprints/Playable/AmericanM_Character_Play` (`GameplayStatics.GetPlayerCharacter` 0)))
  (`self.DisableInput` _asamerican_m_character _returnvalue)
  (`|PlayMontage` (`Character.Mesh` _asamerican_m_character) "/Game/Characters/AmericanM/americanM_kick_Montage.americanM_kick_Montage"
    (:`then`
      (`KismetSystemLibrary.Delay` 0.4)
      (`SceneComponent.SetVisibility` (`self.Object`) false false)
      (`self.Drop Items` (`self.Item To Drop`) (`self.Quantity`)))
    (:`OnCompleted`
      (`self.EnableInput` _asamerican_m_character _returnvalue)
      (`self.K2_DestroyActor`))))

(event `self.Sphere.OnComponentBeginOverlap`
  (params (OverlappedComponent :type "PrimitiveComponent Object Reference") (OtherActor :type "Actor Object Reference") (OtherComp :type "PrimitiveComponent Object Reference") (OtherBodyIndex :type Integer) (bFromSweep :type Boolean) (SweepResult :type "HitResult Structure (by ref)"))
  (bind _asamerican_m_character (cast `/Game/ThirdPerson/Blueprints/Playable/AmericanM_Character_Play` OtherActor))
  (bind _interact_widget (`/Game/ThirdPerson/Blueprints/Playable/AmericanM_Character_Play.Interact Widget` _asamerican_m_character))
  (set `/Game/UI/WBP_Interact.Interact Text` (`self.Interact Text`) _interact_widget)
  (`Widget.SetVisibility` _interact_widget "Visible"))

(event `self.Sphere.OnComponentEndOverlap`
  (params (OverlappedComponent :type "PrimitiveComponent Object Reference") (OtherActor :type "Actor Object Reference") (OtherComp :type "PrimitiveComponent Object Reference") (OtherBodyIndex :type Integer))
  (bind _asamerican_m_character (cast `/Game/ThirdPerson/Blueprints/Playable/AmericanM_Character_Play` OtherActor))
  (`Widget.SetVisibility` (`/Game/ThirdPerson/Blueprints/Playable/AmericanM_Character_Play.Interact Widget` _asamerican_m_character) "Hidden"))

(event `Drop Items`
  (params (`Item To Drop` :type "/Game/Blueprints/Collectables/BP_Collectable Class Reference") (Quantity :type Integer))
  (bind _returnvalue (`KismetMathLibrary.RandomFloatInRange` -20.0 20.0))
  (for _ (range 1 (+ Quantity 1))
    (`|SpawnActorFromClass` `Item To Drop` (`KismetMathLibrary.MakeTransform` (+ (`SceneComponent.K2_GetComponentLocation` (`self.DefaultSceneRoot`)) (`KismetMathLibrary.MakeVector` _returnvalue _returnvalue 50.0))) "Undefined" "OverrideRootScale" null null)))

(fn `Drop Item`
  (params (`Item To Drop` :type "/Game/Blueprints/Collectables/BP_Collectable Class Reference") (Quantity :type Integer)))

(fn `UserConstructionScript`)