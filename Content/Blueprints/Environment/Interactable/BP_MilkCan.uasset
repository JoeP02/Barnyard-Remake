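; Interactable milk can that shows a prompt in range and lets the player collect milk, cream or butter.
; Interact plays fill and pickup montages, attaches a held can to the character and swaps Enhanced Input to milk options.
; Continue advances milk to cream to butter, while Cancel banks the current stage; ShakeComplete only prints pass/fail.
; AddToInventory spawns the collectable to read its item data, adds it to the matching inventory and destroys this actor on success.
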(event `self.Sphere.OnComponentBeginOverlap`
  (params (OverlappedComponent :type "PrimitiveComponent Object Reference") (OtherActor :type "Actor Object Reference") (OtherComp :type "PrimitiveComponent Object Reference") (OtherBodyIndex :type Integer) (bFromSweep :type Boolean) (SweepResult :type "HitResult Structure (by ref)"))
  (bind _asamerican_m_character (cast `/Game/ThirdPerson/Blueprints/Playable/AmericanM_Character_Play` OtherActor))
  (bind _interact_widget (`/Game/ThirdPerson/Blueprints/Playable/AmericanM_Character_Play.Interact Widget` _asamerican_m_character))
  (set `/Game/UI/WBP_Interact.Interact Text` (`self.Interact Text`) _interact_widget)
  (`Widget.SetVisibility` _interact_widget "Visible"))

(event `self.Sphere.OnComponentEndOverlap`
  (params (OverlappedComponent :type "PrimitiveComponent Object Reference") (OtherActor :type "Actor Object Reference") (OtherComp :type "PrimitiveComponent Object Reference") (OtherBodyIndex :type Integer))
  (bind _asamerican_m_character (cast `/Game/ThirdPerson/Blueprints/Playable/AmericanM_Character_Play` OtherActor))
  (`Widget.SetVisibility` (`/Game/ThirdPerson/Blueprints/Playable/AmericanM_Character_Play.Interact Widget` _asamerican_m_character) "Hidden"))

(event `/Game/Blueprints/Interfaces/InteractInterface.Interact`
  (bind _returnvalue (`GameplayStatics.GetPlayerController` 0))
  (`ActorComponent.K2_DestroyComponent` (`self.Sphere`))
  (bind _asamerican_m_character (cast `/Game/ThirdPerson/Blueprints/Playable/AmericanM_Character_Play` (`GameplayStatics.GetPlayerCharacter` 0)))
  (`self.DisableInput` _asamerican_m_character _returnvalue)
  (bind _mesh (`Character.Mesh` _asamerican_m_character))
  (`|PlayMontage` _mesh "/Game/Characters/AmericanM_Barn/americanM_barn_Anim_Urn_fill_Montage.americanM_barn_Anim_Urn_fill_Montage"
    (:`OnCompleted`
      (`|PlayMontage` _mesh "/Game/Characters/AmericanM_Barn/americanM_barn_Anim_Urn_pickUp_Montage.americanM_barn_Anim_Urn_pickUp_Montage"
        (:`then`
          (`SceneComponent.SetVisibility` (`self.SK_Milkcan`) false false)
          (bind _returnvalue_2 (`|SpawnActorFromClass` "/Game/Blueprints/Environment/Non-Destructable/BP_MilkCan_Holding.BP_MilkCan_Holding_C" (`KismetMathLibrary.MakeTransform` (0.0 0.0 0.0) (struct) (0.01 0.01 0.01)) "Undefined" "OverrideRootScale" null null))
          (bind _output_get (set `self.Milkcan` _returnvalue_2))
          (`self.K2_AttachToComponent` _output_get _mesh "CB_RLocator" "KeepRelative" "KeepRelative" "KeepRelative" true))
        (:`OnCompleted`
          (bind _asamerican_m_character_2 (cast `/Game/ThirdPerson/Blueprints/Playable/AmericanM_Character_Play` (`GameplayStatics.GetPlayerCharacter` 0)))
          (set `/Game/ThirdPerson/Blueprints/Playable/AmericanM_Character_Play.bIsHoldingMilkcan` true _asamerican_m_character_2)
          (`self.EnableInput` _asamerican_m_character _returnvalue)
          (`self.EnableInput` _returnvalue)
          (`self.MilkShakeInput` "/Game/Input/IM_MainGame.IM_MainGame" "/Game/Input/IM_MilkOptions.IM_MilkOptions"))))))

(event `MilkShakeInput`
  (params (`Mapping To Remove` :type "InputMappingContext Object Reference") (`Mapping To Add` :type "InputMappingContext Object Reference"))
  (bind _aspc_barnyard_cow (cast `/Game/PC_Barnyard_Cow` (`GameplayStatics.GetPlayerController` 0)))
  (bind _returnvalue (pcsubsystem `EnhancedInputLocalPlayerSubsystem` _aspc_barnyard_cow))
  (`EnhancedInputSubsystemInterface.RemoveMappingContext` _returnvalue `Mapping To Remove` (struct))
  (`EnhancedInputSubsystemInterface.AddMappingContext` _returnvalue `Mapping To Add` 0 (struct))
  (`KismetSystemLibrary.PrintString` "Mapping Stuff"))

(event `EnhancedInput|/Game/Input/MilkingSystem/IA_Continue`
  (params (ActionValue :type Boolean) (ElapsedSeconds :type "Float (double-precision)") (TriggeredSeconds :type "Float (double-precision)") (InputAction :type "InputAction Object Reference" :default "/Game/Input/MilkingSystem/IA_Continue.IA_Continue"))
  (bind _bhasmilk (`self.bHasMilk`))
  (:`Started`
    (`self.MilkShakeInput` "/Game/Input/IM_MilkOptions.IM_MilkOptions" "/Game/Input/IM_Milk.IM_Milk")
    (if (`self.bHasMilk`)
      (set `self.bHasCream` true)
      (`KismetSystemLibrary.PrintString` "Butter")
      (if (and _bhasmilk (`self.bHasCream`)) :!label _label
        (`KismetSystemLibrary.PrintString` "You Got Butter")
        (`self.AddToInventory` "/Game/Blueprints/Collectables/InventoryCollectables/BP_Collectable_Butter.BP_Collectable_Butter_C")
        (elif _bhasmilk
          (`KismetSystemLibrary.PrintString` "You Got Cream")
          (`self.AddToInventory` "/Game/Blueprints/Collectables/InventoryCollectables/BP_Collectable_Cream.BP_Collectable_Cream_C")
          (else
            (`KismetSystemLibrary.PrintString` "You Got Milk")
            (`self.AddToInventory` "/Game/Blueprints/Collectables/InventoryCollectables/BP_Collectable_Milk.BP_Collectable_Milk_C"))))
      (`self.MilkShakeInput` "/Game/Input/IM_MilkOptions.IM_MilkOptions" "/Game/Input/IM_MainGame.IM_MainGame")
      (`self.K2_DestroyActor` (`self.Milkcan`))
      (bind _asamerican_m_character (cast `/Game/ThirdPerson/Blueprints/Playable/AmericanM_Character_Play` (`GameplayStatics.GetPlayerCharacter` 0)))
      (set `/Game/ThirdPerson/Blueprints/Playable/AmericanM_Character_Play.bIsHoldingMilkcan` false _asamerican_m_character)
      (else
        (set `self.bHasMilk` true)
        (`KismetSystemLibrary.PrintString` "Cream")
        (`self.MilkShakeInput` "/Game/Input/IM_Milk.IM_Milk" "/Game/Input/IM_MilkOptions.IM_MilkOptions")))))

(event `EnhancedInput|/Game/Input/MilkingSystem/IA_Cancel`
  (params (ActionValue :type Boolean) (ElapsedSeconds :type "Float (double-precision)") (TriggeredSeconds :type "Float (double-precision)") (InputAction :type "InputAction Object Reference" :default "/Game/Input/MilkingSystem/IA_Cancel.IA_Cancel"))
  (:`Started`
    (goto _label)))

(event `EnhancedInput|/Game/Input/MilkingSystem/IA_Shake`
  (params (ActionValue :type Boolean) (ElapsedSeconds :type "Float (double-precision)") (TriggeredSeconds :type "Float (double-precision)") (InputAction :type "InputAction Object Reference" :default "/Game/Input/MilkingSystem/IA_Shake.IA_Shake")))

(event `ShakeComplete`
  (params (bSuccess :type Boolean))
  (if bSuccess
    (`KismetSystemLibrary.PrintString` "Pass")
    (else
      (`KismetSystemLibrary.PrintString` "Fail"))))

(event `ReturnToGame`)

(fn `AddToInventory`
  (params (ItemData :type "/Game/Blueprints/Collectables/InventoryCollectables/BP_Collectable_Inventory Class Reference"))
  (bind _returnvalue (`|SpawnActorFromClass` ItemData (`KismetMathLibrary.MakeTransform` (0.0 0.0 -500.0)) "Undefined" "OverrideRootScale" null null))
  (bind _asamerican_m_character (cast `/Game/ThirdPerson/Blueprints/Playable/AmericanM_Character_Play` (`GameplayStatics.GetPlayerCharacter` 0)))
  (bind _itemdatacomponent (`/Game/Blueprints/Collectables/InventoryCollectables/BP_Collectable_Inventory.ItemDataComponent` _returnvalue))
  (switch `/Game/Enums/E_InventoryType` (`/Game/Inventory/ItemDataComponent.InventoryType` _itemdatacomponent)
    (:`NewEnumerator0`
      (bind (_itemid_datatable _itemid_rowname) (break `DataTableRowHandle` (`/Game/Inventory/ItemDataComponent.ItemID` _itemdatacomponent)))
      (bind _quantity (`/Game/Inventory/ItemDataComponent.Quantity` _itemdatacomponent))
      (bind _success (`/Game/Inventory/InventoryComponent.AddToInventory` (`/Game/ThirdPerson/Blueprints/Playable/AmericanM_Character_Play.IC_Backpack` _asamerican_m_character) _itemid_rowname _quantity "NewEnumerator0"))
      (if _success
        (`KismetSystemLibrary.PrintString` "Success" :!label _label)
        (`self.K2_DestroyActor`)
        (else
          (`KismetSystemLibrary.PrintString` "Error" :!label _label_2))))
    (:`NewEnumerator1`
      (bind _success_2 (`/Game/Inventory/InventoryComponent.AddToInventory` (`/Game/ThirdPerson/Blueprints/Playable/AmericanM_Character_Play.IC_KnapSack` _asamerican_m_character) _itemid_rowname _quantity "NewEnumerator1"))
      (if _success_2
        (goto _label)
        (else
          (goto _label_2))))
    (:`NewEnumerator2`
      (bind _success_3 (`/Game/Inventory/InventoryComponent.AddToInventory` (`/Game/ThirdPerson/Blueprints/Playable/AmericanM_Character_Play.IC_FlowerPack` _asamerican_m_character) _itemid_rowname _quantity "NewEnumerator2"))
      (if _success_3
        (goto _label)
        (else
          (goto _label_2))))))

(fn `UserConstructionScript`)