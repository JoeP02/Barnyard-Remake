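; GM_OpenWorld is the open-world game mode that broadcasts day and night changes from the sky system's clock.
; BeginPlay finds and stores the BP_EasySkyV2 actor, then, only if found, sets game-only input and hides the cursor.
; Tick polls the sky's hour and minute, setting IsDay and calling IsDayTime or IsNightTime at 7:00 and 19:00.
; The calls have no once-only guard, so they repeat every tick during those minutes.
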(event `self.ReceiveBeginPlay`
  (bind _returnvalue (`GameplayStatics.GetPlayerController` 0))
  (bind _returnvalue_2 (`GameplayStatics.GetActorOfClass` "/EasySkyV2/Blueprints/BP_EasySkyV2.BP_EasySkyV2_C"))
  (`/Engine/EditorBlueprintResources/StandardMacros.IsValid` _returnvalue_2
    (:`Is Valid`
      (set `self.Skybox` _returnvalue_2)
      (`WidgetBlueprintLibrary.SetInputMode_GameOnly` _returnvalue)
      (set `PlayerController.bShowMouseCursor` false _returnvalue))))

(event `self.ReceiveTick`
  (params (DeltaSeconds :type "Float (single-precision)"))
  (bind _skybox (`self.Skybox`))
  (bind _hour (`/EasySkyV2/Blueprints/BP_EasySkyV2.Hour` _skybox))
  (bind _minute (`/EasySkyV2/Blueprints/BP_EasySkyV2.Minute` _skybox))
  (if (and (== _hour 7) (== _minute 0))
    (set `self.IsDay` true)
    (`self.IsDayTime`)
    (elif (and (== _hour 19) (== _minute 0))
      (set `self.IsDay` false)
      (`self.IsNightTime`))))

(fn `UserConstructionScript`
  (`parent.UserConstructionScript`))