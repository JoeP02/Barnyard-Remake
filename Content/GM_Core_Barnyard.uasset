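; Game mode for the Barnyard game that caps the player count and spawns each player as their chosen character.
; PostLogin records joining controllers up to the playercount value parsed from the options string, and tells any extra PC_Core_Barnyard to leave the session in progress.
; New players restart at a found player start, where the SpawnDefaultPawnFor override spawns the character class chosen on their controller.
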(event `self.HandleStartingNewPlayer`
  (params (NewPlayer :type "PlayerController Object Reference"))
  (`self.RestartPlayerAtPlayerStart` NewPlayer (`self.K2_FindPlayerStart` NewPlayer)))

(event `self.K2_PostLogin`
  (params (NewPlayer :type "PlayerController Object Reference"))
  (if (< (`KismetArrayLibrary.Array_Length` (`self.Player List`)) (`KismetStringLibrary.Conv_StringToInt` (`KismetSystemLibrary.ParseParamValue` (`self.OptionsString`) "playercount")))
    (`KismetArrayLibrary.Array_Add` (`self.Player List`) NewPlayer)
    (else
      (bind _aspc_core_barnyard (cast `/Game/PC_Core_Barnyard` NewPlayer))
      (`/Game/PC_Core_Barnyard.LeaveSessionInProgress` _aspc_core_barnyard))))

(fn `SpawnDefaultPawnFor`
  (params (NewPlayer :type "Controller Object Reference") (StartSpot :type "Actor Object Reference"))
  (returns (ReturnValue :type "Pawn Object Reference"))
  (bind _aspc_core_barnyard (cast `/Game/PC_Core_Barnyard` NewPlayer))
  (`/Game/PC_Core_Barnyard.GetCharacterClass` _aspc_core_barnyard)
  (bind _returnvalue (`|SpawnActorFromClass` (`/Game/PC_Core_Barnyard.Chosen Character` _aspc_core_barnyard) (`self.GetTransform` StartSpot) "Undefined" "OverrideRootScale" null null))
  (return _returnvalue))

(fn `UserConstructionScript`)